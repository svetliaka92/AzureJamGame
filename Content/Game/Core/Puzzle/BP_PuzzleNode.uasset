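; BP_PuzzleNode is a puzzle node actor that builds its own set of connection points when play begins.
; For each PointLocations entry it spawns a BP_NodePoint at its location minus that offset, yawed in -90 degree steps, and attaches it to itself.
; The spawned points are collected and handed to SetPoints.
; Clicks on the top and bottom colliders only print the clicked component's name.
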(event `self.ReceiveBeginPlay`
  (bind _pointlocations (`self.PointLocations`))
  (for _index (range (`KismetArrayLibrary.Array_Length` _pointlocations))
    (bind _returnvalue (`|SpawnActorFromClass` "/Game/Game/Core/Puzzle/BP_NodePoint.BP_NodePoint_C" (`KismetMathLibrary.MakeTransform` (- (`self.K2_GetActorLocation`) (`|GetArrayItem` _pointlocations _index)) (`KismetMathLibrary.MakeRotator` 0.0 0.0 (`KismetMathLibrary.Conv_IntToDouble` (`KismetMathLibrary.Round` (`KismetMathLibrary.Conv_IntToDouble` (* _index -90)))))) "Undefined" "OverrideRootScale" null null))
    (`KismetArrayLibrary.Array_Add` (`self.SpawnedPoints`) _returnvalue)
    (`self.K2_AttachToActor` _returnvalue self "None" "KeepWorld" "KeepRelative" "KeepRelative" true))
  (`self.SetPoints` (`self.SpawnedPoints`)))

(event `self.BottomCollider.OnClicked`
  (params (TouchedComponent :type "PrimitiveComponent Object Reference") (ButtonPressed :type "Key Structure"))
  (`KismetSystemLibrary.PrintString` (`KismetSystemLibrary.GetDisplayName` TouchedComponent)))

(event `self.TopCollider.OnClicked`
  (params (TouchedComponent :type "PrimitiveComponent Object Reference") (ButtonPressed :type "Key Structure"))
  (`KismetSystemLibrary.PrintString` (`KismetSystemLibrary.GetDisplayName` TouchedComponent)))

(fn `UserConstructionScript`)