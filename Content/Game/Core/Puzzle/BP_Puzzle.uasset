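; BP_Puzzle is a puzzle manager actor meant to build a grid of BP_PuzzleNode actors.
; CreateGrid spawns nodes across GridSizeX by GridSizeY, spaced by the truncated DistanceBetweenNodes from world origin, then attaches each keeping world location and stores it in Nodes0.
; The CreateGrid and SetNodeGrid chain is disconnected from any event and BeginPlay is empty, so this graph never builds the grid itself.
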(event `self.ReceiveBeginPlay`)

(fn `CreateGrid`
  (returns (Success :type Boolean))
  (bind _returnvalue (`KismetMathLibrary.FTrunc` (`self.DistanceBetweenNodes`)))
  (for _index (range (`self.GridSizeX`))
    (for _index_2 (range (`self.GridSizeY`))
      (bind _returnvalue_2 (`|SpawnActorFromClass` "/Game/Game/Core/Puzzle/BP_PuzzleNode.BP_PuzzleNode_C" (`KismetMathLibrary.MakeTransform` (`KismetMathLibrary.MakeVector` (`KismetMathLibrary.Conv_IntToDouble` (* _index _returnvalue)) (`KismetMathLibrary.Conv_IntToDouble` (* _index_2 _returnvalue)))) "Undefined" "OverrideRootScale" null null))
      (`self.K2_AttachToActor` _returnvalue_2 self "None" "KeepWorld" "KeepRelative" "KeepRelative" true)
      (bind _asbp_puzzle_node (cast `/Game/Game/Core/Puzzle/BP_PuzzleNode` _returnvalue_2))
      (`KismetArrayLibrary.Array_Add` (`self.Nodes_0`) _asbp_puzzle_node)))
  (return true))

(fn `UserConstructionScript`)